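; Camera actor that starts the car crash cutscene when the first person character enters its trigger box.
; On overlap it disables the player's input and quickly blends the view to itself.
; After short staggered delays it plays the CarCrash level sequence, adds the FALLBLACK_WBP widget to the viewport and sets the CutScenePlay flag.
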(event OnComponentBeginOverlap(Box)
  (params (OverlappedComponent :type Primitive%20Component%20Object%20Reference) (OtherActor :type Actor%20Object%20Reference) (OtherComp :type Primitive%20Component%20Object%20Reference) (OtherBodyIndex :type Integer) (bFromSweep :type Boolean) (SweepResult :type Hit%20Result%20Structure%20%28by%20ref%29))
  (bind _asfirst_person_character (Utilities|Casting|CastToFirstPersonCharacter OtherActor))
  (Input|DisableInput _asfirst_person_character (Game|GetPlayerController 0))
  (Game|Player|SetViewTargetwithBlend (Game|GetPlayerController 0) self 0.1 "VTBlend_Linear" 0.0 false)
  (Utilities|FlowControl|Sequence
    (:then_0
      (Utilities|FlowControl|Delay 0.1)
      (bind _returnvalue (Sequencer|Player|CreateLevelSequencePlayer "/Game/CarCrash.CarCrash"))
      (Sequencer|Player|Play _returnvalue :!class /Script/MovieScene.MovieSceneSequencePlayer))
    (:then_1
      (Utilities|FlowControl|Delay 0.2)
      (bind _returnvalue_2 (UserInterface|CreateWidget "/Game/UI/FALLBLACK_WBP.FALLBLACK_WBP_C"))
      (UserInterface|Viewport|AddtoViewport _returnvalue_2 0)
      (Variables|Default|SetCutScene_Play? true))))

(fn ConstructionScript)